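; BP_Mage is a top-down-style player mage pawn that moves on world axes, aims independently and adds W_PlayerHUD on BeginPlay.
; Each tick sets control rotation from thumbstick direction or smoothed mouse velocity, both deadzone-gated, chosen by whether the last key pressed was gamepad.
; FireWeapon spawns a delayed burst of four BP_Fireballs at a fixed world offset with the actor's rotation.
; The FireSpell function is left unused.
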(event EventBeginPlay
  (bind _returnvalue (UserInterface|CreateWidget "/Game/UI/W_PlayerHud.W_PlayerHUD_C" 0 self))
  (UserInterface|Viewport|AddtoViewport _returnvalue 0))

(event Collision|EventActorBeginOverlap
  (params (OtherActor :type Actor%20Object%20Reference)))

(event EventTick
  (params (DeltaSeconds :type Float%20%28single-precision%29))
  (CallFunction|UpdatePlayerAim))

(event Input|ActionEvents|InputActionFireWeapon
  (params (Key :type Key%20Structure :default "None"))
  (bind _returnvalue (Transformation|GetActorTransform))
  (bind (_location _rotation _scale) (Math|Transform|BreakTransform _returnvalue))
  (:Pressed
    (Utilities|DelayedforLoop 0 3 0.3
      (:Loop%20Body
        (Game|SpawnActorfromClass "/Game/Characters/Marine/Spells/BP_Fireball.BP_Fireball_C" (Math|Transform|MakeTransform (+ _location "0,25.000000,35.000000") _rotation _scale) "AlwaysSpawn" 0 0)))))

(event Input|AxisEvents|InputAxisMoivngForward
  (params (AxisValue :type Float%20%28single-precision%29))
  (Pawn|Input|AddMovementInput "1.000000, 0, 0" AxisValue false))

(event Input|AxisEvents|InputAxisMoivngRight
  (params (AxisValue :type Float%20%28single-precision%29))
  (Pawn|Input|AddMovementInput "0.000000,1.000000, 0" AxisValue false))

(event Input|KeyboardEvents|AnyKey
  (params (Key :type Key%20Structure :default "None"))
  (:Pressed
    (Variables|Default|SetKeyIsGamepad (Class|KismetInputLibrary|KeyIsGamepadKey Key))))

(fn ConstructionScript)

(fn UpdatePlayerAim
  (if (Variables|Default|GetKeyIsGamepad)
    (ThumbstickInput|UpdateThumbstickAIm)
    (else
      (MouseInput|MouseAimUpdate))))

(fn IsFunctuionAboveDeadzone
  (return (> (Math|Vector2D|Vector2DLength (Math|Vector2D|MakeVector2D (Input|AxisValues|GetThumbstickAImUp) (Input|AxisValues|GetThumbstickAimRight))) (LocalVariables|GetThumbstickDeadzone))))

(fn GetMouseVelocity
  (bind _returnvalue (Game|GetPlayerController 0))
  (bind (_deltax _deltay) (Class|PlayerController|GetInputMouseDelta _returnvalue))
  (return (/ (Math|Vector2D|MakeVector2D _deltax _deltay) (Utilities|Time|GetWorldDeltaSeconds))))

(fn IsMouseAboveDeadzone
  (return (> (Math|Vector2D|Vector2DLength (MouseInput|GetMouseVelocity)) (LocalVariables|GetMouseDeadzone))))

(fn MouseAimUpdate
  (if (MouseInput|IsMouseAboveDeadzone)
    (Pawn|SetControlRotation (Game|GetPlayerController 0) (MouseInput|UpdateMouseAim))))

(fn UpdateMouseAim
  (bind _returnvalue (MouseInput|GetMouseVelocity))
  (return (Math|Interpolation|RInterpTo (Pawn|GetControlRotation (Game|GetPlayerController 0) :!class /Script/Engine.Controller) (Math|Rotator|MakeRotator 0.0 0.0 (Class|KismetMathLibrary|DegAtan2 (.x _returnvalue) (.y _returnvalue))) (Utilities|Time|GetWorldDeltaSeconds) (LocalVariables|GetAimSmoothing))))

(fn GetThumbstickAimDirection
  (return (Math|Rotator|MakeRotator 0.0 0.0 (Class|KismetMathLibrary|DegAtan2 (Input|AxisValues|GetThumbstickAimRight) (Input|AxisValues|GetThumbstickAImUp)))))

(fn UpdateThumbstickAIm
  (if (ThumbstickInput|IsFunctuionAboveDeadzone)
    (Pawn|SetControlRotation (Game|GetPlayerController 0) (ThumbstickInput|GetThumbstickAimDirection))))

(fn FireSpell
  (bind _returnvalue (Transformation|GetActorTransform))
  (bind (_location _rotation _scale) (Math|Transform|BreakTransform _returnvalue))
  (for _index (range 0 4 0.0)
    (Game|SpawnActorfromClass "/Game/Characters/Marine/Spells/BP_Fireball.BP_Fireball_C" (Math|Transform|MakeTransform (+ _location "0,25.000000,35.000000") _rotation _scale) "AlwaysSpawn" 0 0)))